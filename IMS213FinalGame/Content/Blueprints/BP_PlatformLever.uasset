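; Interactable lever that spawns a set of temporary platforms at preset transforms for a limited time.
; Overlapping its sphere shows an interact widget; interacting spawns the platforms, resets the player character's Seconds counter and adds a W_TimeLimit widget.
; A looping one-second timer decrements that counter, and at zero it removes the widget, clears the timer and destroys every BP_SpawnedPlatform in the world.
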(event `/Game/Blueprints/BPI_Interact.Interact`
  (`self.Create Platforms`)
  (bind _asbp_third_person_character (cast `/Game/ThirdPerson/Blueprints/BP_ThirdPersonCharacter` (`GameplayStatics.GetPlayerCharacter` 0)))
  (set `/Game/ThirdPerson/Blueprints/BP_ThirdPersonCharacter.Seconds` 20 _asbp_third_person_character)
  (set `self.ContinueCountdown` true)
  (`self.Start Platform Time Countdown`))

(event `self.Sphere.OnComponentBeginOverlap`
  (params (OverlappedComponent :type "PrimitiveComponent Object Reference") (OtherActor :type "Actor Object Reference") (OtherComp :type "PrimitiveComponent Object Reference") (OtherBodyIndex :type Integer) (bFromSweep :type Boolean) (SweepResult :type "HitResult Structure (by ref)"))
  ;[1 1 1] Interaction Widget Visibility
  (`SceneComponent.SetVisibility` (`self.LeverInteractWidget`) true false))

(event `Start Platform Time Countdown`
  ;[1 1 1] Platform Seconds Countdown
  (bind _returnvalue (`|CreateWidget` "/Game/Blueprints/W_TimeLimit.W_TimeLimit_C"))
  (`UserWidget.AddToViewport` _returnvalue 0)
  (bind _returnvalue_2 (`KismetSystemLibrary.K2_SetTimerDelegate` (delegate `Countdown Seconds`) 1.0 (`self.ContinueCountdown`))))

(event `self.Sphere.OnComponentEndOverlap`
  (params (OverlappedComponent :type "PrimitiveComponent Object Reference") (OtherActor :type "Actor Object Reference") (OtherComp :type "PrimitiveComponent Object Reference") (OtherBodyIndex :type Integer))
  ;[1 1 1] Interaction Widget Visibility
  (`SceneComponent.SetVisibility` (`self.LeverInteractWidget`) false false))

(event `Countdown Seconds`
  ;[1 1 1] Platform Seconds Countdown
  (bind _asbp_third_person_character (cast `/Game/ThirdPerson/Blueprints/BP_ThirdPersonCharacter` (`GameplayStatics.GetPlayerCharacter` 0)))
  (if (== (`/Game/ThirdPerson/Blueprints/BP_ThirdPersonCharacter.Seconds` _asbp_third_person_character) 0)
    (set `self.ContinueCountdown` false)
    (bind _foundwidgets (`WidgetBlueprintLibrary.GetAllWidgetsOfClass` "/Game/Blueprints/W_TimeLimit.W_TimeLimit_C"))
    (`Widget.RemoveFromParent` _foundwidgets)
    (`KismetSystemLibrary.K2_ClearAndInvalidateTimerHandle` (stale `Start Platform Time Countdown` _returnvalue_2))
    (bind _outactors (`GameplayStatics.GetAllActorsOfClass` "/Game/Blueprints/BP_SpawnedPlatform.BP_SpawnedPlatform_C"))
    (for _array_element _outactors
      (`self.K2_DestroyActor` _array_element))
    (else
      (set `/Game/ThirdPerson/Blueprints/BP_ThirdPersonCharacter.Seconds` (- (`/Game/ThirdPerson/Blueprints/BP_ThirdPersonCharacter.Seconds` _asbp_third_person_character) 1) _asbp_third_person_character))))

(event `Create Platforms`
  ;[1 1 1] Create 9 Limited-Time Platforms
  (`|SpawnActorFromClass` "/Game/Blueprints/BP_SpawnedPlatform.BP_SpawnedPlatform_C" (`self.Platform1_Position`) "Undefined" "MultiplyWithRoot" null null)
  (`|SpawnActorFromClass` "/Game/Blueprints/BP_SpawnedPlatform.BP_SpawnedPlatform_C" (`self.Platform2_Position`) "Undefined" "MultiplyWithRoot" null null)
  (`|SpawnActorFromClass` "/Game/Blueprints/BP_SpawnedPlatform.BP_SpawnedPlatform_C" (`self.Platform3_Position`) "Undefined" "MultiplyWithRoot" null null)
  (`|SpawnActorFromClass` "/Game/Blueprints/BP_SpawnedPlatform.BP_SpawnedPlatform_C" (`self.Platform4_Position`) "Undefined" "MultiplyWithRoot" null null)
  (`|SpawnActorFromClass` "/Game/Blueprints/BP_SpawnedPlatform.BP_SpawnedPlatform_C" (`self.Platform5_Position`) "Undefined" "MultiplyWithRoot" null null)
  (`|SpawnActorFromClass` "/Game/Blueprints/BP_SpawnedPlatform.BP_SpawnedPlatform_C" (`self.Platform6_Position`) "Undefined" "MultiplyWithRoot" null null)
  (`|SpawnActorFromClass` "/Game/Blueprints/BP_SpawnedPlatform.BP_SpawnedPlatform_C" (`self.Platform7_Position`) "Undefined" "MultiplyWithRoot" null null)
  (`|SpawnActorFromClass` "/Game/Blueprints/BP_SpawnedPlatform.BP_SpawnedPlatform_C" (`self.Platform8_Position`) "Undefined" "MultiplyWithRoot" null null)
  (`|SpawnActorFromClass` "/Game/Blueprints/BP_SpawnedPlatform.BP_SpawnedPlatform_C" (`self.Platform9_Position`) "Undefined" "MultiplyWithRoot" null null))

(fn `UserConstructionScript`)