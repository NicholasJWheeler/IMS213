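; BP_Door is a locked door that the player can open and close with Interact once a key has been picked up.
; PickUpKey sets HasKey and destroys the lock component.
; With the key, Interact flip-flops a timeline that plays or reverses to swing the door mesh's yaw between closed and open.
; Overlapping the box shows either an interact or need-key prompt based on HasKey, and leaving hides both.
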(event `/Game/Blueprints/BPI_Interact.Interact`
  (if (`self.HasKey?`)
    (`/Engine/EditorBlueprintResources/StandardMacros.FlipFlop`
      (:`A`
        (bind (_direction _doortrack) (`Timeline|Door Timeline` :!label _label)
          (:`Update`
            (`SceneComponent.K2_SetRelativeRotation` (`self.SM_Door`) (`KismetMathLibrary.MakeRotator` 0.0 0.0 (`KismetMathLibrary.Lerp` 0.0 110.0 _doortrack)) false false))))
      (:`B`
        (goto _label :!via `Reverse`)))))

(event `/Game/Blueprints/BPI_Door.Pick Up Key`
  (set `self.HasKey?` true)
  (`ActorComponent.K2_DestroyComponent` (`self.lock_lock`)))

(event `self.Box.OnComponentBeginOverlap`
  (params (OverlappedComponent :type "PrimitiveComponent Object Reference") (OtherActor :type "Actor Object Reference") (OtherComp :type "PrimitiveComponent Object Reference") (OtherBodyIndex :type Integer) (bFromSweep :type Boolean) (SweepResult :type "HitResult Structure (by ref)"))
  (if (`self.HasKey?`)
    (`SceneComponent.SetVisibility` (`self.DoorInteractWidget`) true false)
    (else
      (`SceneComponent.SetVisibility` (`self.NeedKeyWidget`) true false))))

(event `self.Box.OnComponentEndOverlap`
  (params (OverlappedComponent :type "PrimitiveComponent Object Reference") (OtherActor :type "Actor Object Reference") (OtherComp :type "PrimitiveComponent Object Reference") (OtherBodyIndex :type Integer))
  (`SceneComponent.SetVisibility` (`self.DoorInteractWidget`) false false)
  (`SceneComponent.SetVisibility` (`self.NeedKeyWidget`) false false))

(fn `UserConstructionScript`)